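; BP_BuildSource is a building Blueprint that displays its base resource amount in the world.
; On BeginPlay it runs the parent logic, then writes BaseResources as an integer to its TextRender component once.
; Tick and the construction script only call the parent, and the overlap event is disabled, so this graph adds no other behavior.
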(event `self.ReceiveBeginPlay`
  (`parent.ReceiveBeginPlay`)
  (`TextRenderComponent.K2_SetText` (`self.TextRender`) (`KismetTextLibrary.Conv_IntToText` (`self.BaseResources`))))

(event `self.ReceiveTick`
  (params (DeltaSeconds :type "Float (single-precision)"))
  (`parent.ReceiveTick` DeltaSeconds))

(fn `UserConstructionScript`
  (`parent.UserConstructionScript`))