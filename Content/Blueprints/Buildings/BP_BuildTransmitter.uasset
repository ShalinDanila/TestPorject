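; Transmitter building that draws resources from nearby placed buildings and shows its stored amount as text.
; Each Tick it takes one unit from the current target, a source or another transmitter, then re-searches the player's PlacedMesh list for the nearest building within range.
; It separately gains one unit while a building is found and capacity remains, even if that target is empty, and drains the target even when full.
; An anchor arrow yaws along the target-to-transmitter line.
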(event `self.ReceiveBeginPlay`
  ;[0.3302 0.3302 0.3302 0.454] Инициализация переменных
  (`parent.ReceiveBeginPlay`)
  (bind _returnvalue (`GameplayStatics.GetActorOfClass` "/Game/Blueprints/FirstPersonCharacter.FirstPersonCharacter_C"))
  (set `self.FirstPersonRef` _returnvalue)
  (bind _returnvalue_2 (`GameplayStatics.GetActorOfClass` "/Game/Blueprints/Buildings/BP_BuildSource.BP_BuildSource_C"))
  (set `self.BuildRef` _returnvalue_2))

(event `self.ReceiveTick`
  (params (DeltaSeconds :type "Float (single-precision)"))
  (bind _ancher (`self.Ancher`))
  (bind _resourcesamount (`self.ResourcesAmount`))
  ;[0.3302 0.3302 0.3302 0.454] Поиск не пустого источника ресурсов
  (`|ExecutionSequence`
    (:`then_0`
      (`parent.ReceiveTick` DeltaSeconds)
      (`|ExecutionSequence`
        (:`then_0`
          ;[0.3302 0.3302 0.3302 0.454] Изменение значения ресурсов у здания цели
          (bind _asbp_build_source (cast `/Game/Blueprints/Buildings/BP_BuildSource` (`self.BuildRef`))
            (:`then`
              (bind _baseresources (`/Game/Blueprints/Buildings/BP_BuildSource.BaseResources` _asbp_build_source))
              (if (not (<= _baseresources 0))
                (bind _output_get (set `/Game/Blueprints/Buildings/BP_BuildSource.BaseResources` (- _baseresources 1) _asbp_build_source))
                (`TextRenderComponent.K2_SetText` (`/Game/Blueprints/Buildings/BP_BuildSource.TextRender` _asbp_build_source) (`KismetTextLibrary.Conv_IntToText` _output_get))))
            (:`CastFailed`
              (bind _asbp_build_transmitter (cast `/Game/Blueprints/Buildings/BP_BuildTransmitter` (`self.BuildRef`)))
              (bind _resourcesamount_2 (`/Game/Blueprints/Buildings/BP_BuildTransmitter.ResourcesAmount` _asbp_build_transmitter))
              (if (not (<= _resourcesamount_2 0))
                (set `/Game/Blueprints/Buildings/BP_BuildTransmitter.ResourcesAmount` (- _resourcesamount_2 1) _asbp_build_transmitter)))))
        (:`then_1`
          (bind (_nearestbuilding _returnvalue) (`self.FindNearestBuilding`))
          (set `self.BuildRef` _nearestbuilding)
          (set `self.BuildingWasFound` _returnvalue))))
    (:`then_1`
      ;[0.3302 0.3302 0.3302 0.454] Изменение значения ресурсов передатчика
      (if (and (`self.BuildingWasFound`) (< _resourcesamount (`self.MaxResourcesAmount`)))
        (bind _output_get_2 (set `self.ResourcesAmount` (+ _resourcesamount 1)))
        (`TextRenderComponent.K2_SetText` (`self.TextRender`) (`KismetTextLibrary.Conv_IntToText` _output_get_2))
        (else
          (set `self.TransmitterIsFull` true))))
    (:`then_2`
      ;[0.3302 0.3302 0.3302 0.454] Поворот стрелки в сторону источника
      (bind _buildref (`self.BuildRef`)
        (:`then`
          (bind (_returnvalue_roll _returnvalue_pitch _returnvalue_yaw) (`KismetMathLibrary.BreakRotator` (`KismetMathLibrary.FindLookAtRotation` (`self.K2_GetActorLocation` _buildref) (`SceneComponent.K2_GetComponentLocation` _ancher))))
          (`SceneComponent.K2_SetRelativeRotation` _ancher (`KismetMathLibrary.MakeRotator` 0.0 0.0 _returnvalue_yaw) false false))
        (:`else`)))))

(fn `FindNearestBuilding`
  (returns (NearestBuilding :type "Actor Object Reference") (ReturnValue :type Boolean))
  (bind _returnvalue (< (`self.NearestDist`) 1000.0))
  (bind _placedmesh (`/Game/Blueprints/FirstPersonCharacter.PlacedMesh` (`self.FirstPersonRef`)))
  ;[0.3302 0.3302 0.3302 0.454] Ищем ближайший объект
  (for (_array_element _array_index) _placedmesh
    (bind _returnvalue_2 (`KismetMathLibrary.VSize` (- (`self.K2_GetActorLocation` _array_element) (`self.K2_GetActorLocation`))))
    ;;[0.3302 0.3302 0.3302 0.454] Поиск индекса ближайшего объекта
    (if (and (< _returnvalue_2 (`self.NearestDist`)) (> _returnvalue_2 1.0))
      (set `self.NearestDist` _returnvalue_2)
      (set `self.NearestIndex` _array_index)))
  ;;[0.3302 0.3302 0.3302 0.454] Записываем индекс ближайшего объекта
  (if _returnvalue
    (return (`|GetArrayItem` _placedmesh (`self.NearestIndex`)) _returnvalue)
    (else
      (return null false))))

(fn `FindSources`
  (returns (SourceRef :type "Actor Object Reference") (ReturnValue :type Integer))
  (bind _output_get (set `self.BuildRef` null)))

(fn `UserConstructionScript`
  (`parent.UserConstructionScript`))