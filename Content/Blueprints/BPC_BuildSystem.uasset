(event `self.ReceiveTick`
  (params (DeltaSeconds :type "Float (single-precision)"))
  (if (`self.InBuildMode?`)
    (`self.Preview Loop`)))

(event `self.ReceiveBeginPlay`
  ;[0.3302 0.3302 0.3302 0.454] Инициализация переменных
  (bind _returnvalue (`GameplayStatics.GetActorOfClass` "/Game/Blueprints/FirstPersonCharacter.FirstPersonCharacter_C"))
  (set `self.First Person Character` _returnvalue)
  (set `self.First Person Camera` (`/Game/Blueprints/FirstPersonCharacter.FirstPersonCamera` _returnvalue))
  ;[0.3302 0.3302 0.3302 0.454] Инициализация возможных построек
  (bind _outrownames (`DataTableFunctionLibrary.GetDataTableRowNames` "/Game/Blueprints/Buildings/DT_BuildData.DT_BuildData"))
  (for _array_element _outrownames
    (bind _returnvalue_2 (`|GetDataTableRow` "/Game/Blueprints/Buildings/DT_BuildData.DT_BuildData" _array_element)
      (:`then`
        (`KismetArrayLibrary.Array_Add` (`self.BuildingsDataTable`) _returnvalue_2)))))

(event `Preview Loop`
  (bind _previewmesh (`self.PreviewMesh`))
  (bind (_returnvalue_location _returnvalue_rotation) (`KismetMathLibrary.BreakTransform` (`SceneComponent.K2_GetComponentToWorld` (`self.First Person Camera`))))
  ;[0.3302 0.3302 0.3302 0.454] Предпросмотр объекта перед постройкой
  (bind (_outhit _returnvalue) (`KismetSystemLibrary.LineTraceSingle` _returnvalue_location (+ _returnvalue_location (* (`KismetMathLibrary.GetForwardVector` _returnvalue_rotation) 700.0)) "TraceTypeQuery1"))
  (if _returnvalue
    (`|ExecutionSequence`
      (:`then_0`
        (`/Engine/EditorBlueprintResources/StandardMacros.DoOnce` false :!label _label
          (:`Completed`
            (bind _returnvalue_2 (`|AddComponentByClass` (`self.First Person Character`) "/Script/Engine.StaticMeshComponent" false (`self.BuildPreviewTransform`)))
            (bind _output_get (set `self.PreviewMesh` _returnvalue_2))
            (`StaticMeshComponent.SetStaticMesh` _output_get (`.Mesh_8_3681D13E43EFD914E4FE37872E9F436A` (break `/Game/Blueprints/Buildings/S_Buildings` (`|GetArrayItem` (`self.BuildingsDataTable`) (`self.BuildingsIndex`)))))
            (`PrimitiveComponent.SetMaterial` _previewmesh 0 "/Game/Material/M_PreviewMaterial.M_PreviewMaterial")
            (`PrimitiveComponent.SetCollisionEnabled` _previewmesh "NoCollision"))))
      (:`then_1`
        (bind _output_get_2 (set `self.BuildPreviewTransform` (`KismetMathLibrary.MakeTransform` (`.Location` (`GameplayStatics.BreakHitResult` _outhit)))))
        (`SceneComponent.K2_SetWorldTransform` (`self.PreviewMesh`) _output_get_2 false false)))))

(event `Reset Build Mode`
  ;[0.3302 0.3302 0.3302 0.454] Предпросмотр объекта перед постройкой
  (goto _label :!via `Reset`))